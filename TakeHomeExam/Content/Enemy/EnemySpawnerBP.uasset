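; Enemy spawner actor that keeps filling its box volume with AI enemies while the game's enemy count stays low.
; On BeginPlay it caches the ShooterGameMode and starts a looping half-second timer.
; Each tick of the timer checks the game mode's enemy count against a cap, spawns an EnemyBP at a random point in the scaled box, and increments that shared count.
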(event Custom|SpawnEnemy
  (bind _gamemode (Variables|Default|GetGameMode))
  (bind _box (Variables|Default|GetBox))
  (if (<= (Variables|/Game/ShooterGameMode.ShooterGameMode_C|GetNumberEnemies _gamemode) 10)
    (AI|SpawnAIFromClass "/Game/Enemy/EnemyBP.EnemyBP_C" 0 (Math|Random|RandomPointinBoundingBox (Transformation|GetWorldLocation _box) (Components|Box|GetScaledBoxExtent _box)) "0, 0, 0" false)
    (Default|IncreaseNumberEnemies _gamemode)))

(event EventBeginPlay
  (bind _asshooter_game_mode (Utilities|Casting|CastToShooterGameMode (Game|GetGameMode)))
  (Variables|Default|SetGameMode _asshooter_game_mode)
  (Utilities|Time|SetTimerbyFunctionName 0 "SpawnEnemy" 0.5 true))

(event Collision|EventActorBeginOverlap
  (params (OtherActor :type Actor%20Object%20Reference)))

(event EventTick
  (params (DeltaSeconds :type Float%20%28single-precision%29)))

(fn ConstructionScript)