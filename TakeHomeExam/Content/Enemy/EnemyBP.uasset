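; Enemy actor that damages the hero on contact and can be killed to advance score in the shooter game mode.
; Overlap with HeroBP deals damage at once and starts a looping timer that repeats it until the overlap ends.
; Its DecreaseHP event lowers health and, at zero, tells the cached ShooterGameMode to lower the enemy count and raise score, then destroys the actor.
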(event Custom|DecreaseHeroHP
  (Class|DamagedInterface|DecreaseHP(Message) (stale Collision|EventActorBeginOverlap _ashero_bp) 2e+01))

(event EventBeginPlay
  (Variables|Default|SetHp 1e+02)
  (bind _asshooter_game_mode (Utilities|Casting|CastToShooterGameMode (Game|GetGameMode)))
  (Variables|Default|SetGameMode _asshooter_game_mode))

(event Collision|EventActorBeginOverlap
  (params (OtherActor :type Actor%20Object%20Reference))
  (bind _ashero_bp (Utilities|Casting|CastToHeroBP OtherActor))
  (CallFunction|DecreaseHeroHP)
  (Utilities|Time|SetTimerbyFunctionName 0 "DecreaseHeroHP" 0.2 true))

(event Collision|EventActorEndOverlap
  (params (OtherActor :type Actor%20Object%20Reference))
  (Utilities|Casting|CastToHeroBP OtherActor)
  (Utilities|Time|ClearTimerbyFunctionName 0 "DecreaseHeroHP"))

(event EventTick
  (params (DeltaSeconds :type Float%20%28single-precision%29)))

(event EventDecreaseHP
  (params (amount :type Float%20%28single-precision%29))
  (bind _gamemode (Variables|Default|GetGameMode))
  (bind _output_get (Variables|Default|SetHp (- (Variables|Default|GetHp) amount)))
  (if (<= _output_get 0.0)
    (Default|DecreaseNumberEnemies _gamemode)
    (Default|IncreaseScore _gamemode)
    (Actor|DestroyActor)))

(fn ConstructionScript)