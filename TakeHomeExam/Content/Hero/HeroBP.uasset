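; Player hero pawn that moves along world axes, fires an attached gun and tracks health.
; On BeginPlay it spawns a GunBP on the mesh's GunPoint socket and caches the ShooterGameMode, while trigger input starts and stops firing.
; Both turn axes share logic that sets rotation from the input vector outside a small dead zone.
; DecreaseHP updates the game mode's UI and, at zero health, destroys hero and gun and restarts the level.
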(event EventBeginPlay
  (Variables|Default|SetHp 1e+02)
  (bind _asshooter_game_mode (Utilities|Casting|CastToShooterGameMode (Game|GetGameMode)))
  (Variables|Default|SetGameMode _asshooter_game_mode)
  (bind _returnvalue (Game|SpawnActorfromClass "/Game/Gun/GunBP.GunBP_C" (Transformation|GetWorldTransform (Variables|Character|GetMesh)) "Undefined" 0 0))
  (bind _output_get (Variables|Default|SetGun _returnvalue))
  (Transformation|AttachComponentToComponent _output_get (Variables|Character|GetMesh) "GunPoint" "SnapToTarget" "SnapToTarget" "SnapToTarget" true))

(event Collision|EventActorBeginOverlap
  (params (OtherActor :type Actor%20Object%20Reference)))

(event EventTick
  (params (DeltaSeconds :type Float%20%28single-precision%29)))

(event EventDecreaseHP
  (params (amount :type Float%20%28single-precision%29))
  (bind _output_get (Variables|Default|Sethp (- (Variables|Default|Gethp) amount)))
  (Default|UpdateHeroHP (Variables|/Game/ShooterGameMode.ShooterGameMode_C|GetGameUI (Variables|Default|GetGameMode)))
  (if (<= _output_get 0.0)
    (Input|DisableInput 0)
    (Actor|DestroyActor (Variables|Default|GetGun))
    (Development|ExecuteConsoleCommand "restartlevel")))

(event Input|ActionEvents|InputActionTriggerBullet
  (params (Key :type Key%20Structure :default "AnyKey"))
  (bind _gun (Variables|Default|GetGun))
  (:Pressed
    (Default|StartFiring _gun))
  (:Released
    (Default|StopFiring _gun)))

(event Input|AxisEvents|InputAxisMoveForward
  (params (AxisValue :type Float%20%28single-precision%29))
  (Pawn|Input|AddMovementInput "1.000000, 0, 0" AxisValue false))

(event Input|AxisEvents|InputAxisTurnUP
  (params (AxisValue :type Float%20%28single-precision%29))
  (if (not (Math|Float|NearlyEqual(Float) (Math|Vector|VectorLengthSquared (Math|Vector|MakeVector AxisValue (stale Input|AxisEvents|InputAxisTurnLeft AxisValue) 0.0)) 0.0 0.01))
    (Transformation|SetActorRotation (Math|Conversions|RotationFromXVector (Math|Vector|MakeVector AxisValue (stale Input|AxisEvents|InputAxisTurnLeft AxisValue) 0.0)))))

(event Input|AxisEvents|InputAxisTurnLeft
  (params (AxisValue :type Float%20%28single-precision%29))
  (if (not (Math|Float|NearlyEqual(Float) (Math|Vector|VectorLengthSquared (Math|Vector|MakeVector (stale Input|AxisEvents|InputAxisTurnUP AxisValue) AxisValue 0.0)) 0.0 0.01))
    (Transformation|SetActorRotation (Math|Conversions|RotationFromXVector (Math|Vector|MakeVector (stale Input|AxisEvents|InputAxisTurnUP AxisValue) AxisValue 0.0)))))

(event Input|AxisEvents|InputAxisMoveRight
  (params (AxisValue :type Float%20%28single-precision%29))
  (Pawn|Input|AddMovementInput "0.000000,1.000000, 0" AxisValue false))

(fn ConstructionScript)